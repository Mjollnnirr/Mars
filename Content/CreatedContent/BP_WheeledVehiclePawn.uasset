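; Wheeled vehicle pawn with a grapple move, fired by right mouse, that pulls the vehicle toward whatever the front camera faces.
; A visibility sphere trace runs forward from the Rover_Pawn's FrontCamera, with debug drawing, and passes a slightly pulled-back hit point to the Grappling event.
; Grappling plays a timeline that lerps the actor from its starting location to that point, teleporting without sweep.
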(event `Key|RightMouseButton`
  (params (Key :type "Key Structure"))
  (:`Pressed`
    (bind _newparam (`self.GetFrontCamera`))
    (bind _returnvalue (`SceneComponent.K2_GetComponentLocation` _newparam))
    (bind _returnvalue_2 (`SceneComponent.GetForwardVector` _newparam))
    (bind (_outhit _returnvalue_3) (`KismetSystemLibrary.SphereTraceSingle` :`Start` _returnvalue :`End` (+ _returnvalue (* _returnvalue_2 2000.0)) :`TraceChannel` "TraceTypeQuery1" :`DrawDebugType` "ForDuration"))
    (if _returnvalue_3
      (`self.Grappling` (+ (`.Location` (`GameplayStatics.BreakHitResult` _outhit)) (* _returnvalue_2 -56.0))))))

(event `Grappling`
  (params (AttachPoint :type "Vector Structure"))
  (set `self.StartPoint` (`self.K2_GetActorLocation`))
  (bind (_direction _alpha) (`Timeline|Grapple` :!via `PlayFromStart`)
    (:`Update`
      (`self.K2_SetActorLocation` (`KismetMathLibrary.VLerp` (`self.StartPoint`) AttachPoint _alpha) false true))))

(fn `GetFrontCamera`
  (returns (NewParam :type "CameraComponent Object Reference"))
  (bind _asrover_pawn (cast `/Game/Rover/Rover_Pawn` (`PawnMovementComponent.GetPawnOwner` (`self.VehicleMovementComponent`))))
  (return (`/Game/Rover/Rover_Pawn.FrontCamera` _asrover_pawn)))

(fn `UserConstructionScript`)