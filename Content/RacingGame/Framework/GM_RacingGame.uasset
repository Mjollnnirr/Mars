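; Racing game mode that runs a timed checkpoint race, printing Win or Lose at the end.
; On BeginPlay it binds to every BP_Checkpoint, treating finish lines separately from timed checkpoints, then starts a countdown delay.
; A one-shot timer then triggers the out-of-time loss, and the finish-line win clears it.
; Checkpoint time is added only to the StartTimerDuration variable, without resetting the running timer.
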(event `self.ReceiveBeginPlay`
  (`|ExecutionSequence`
    (:`then_0`
      (bind _outactors (`GameplayStatics.GetAllActorsOfClass` "/Game/RacingGame/Checkpoints/BP_Checkpoint.BP_Checkpoint_C"))
      (for _array_element _outactors
        (if (`/Game/RacingGame/Checkpoints/BP_Checkpoint.bFinishLine` _array_element)
          (add `/Game/RacingGame/Checkpoints/BP_Checkpoint.OnCheckpointCrossed` _array_element (`|CreateDelegate` :!event `WinCrossedFinishLine`))
          (else
            (add `/Game/RacingGame/Checkpoints/BP_Checkpoint.OnCheckpointCrossedWithTime` _array_element (`|CreateDelegate` :!event `CrossedCheckpoint`))))))
    (:`then_1`
      (`self.Start Countdown`))))

(event `Start Countdown`
  (`KismetSystemLibrary.Delay` (`self.StartCountdownDuration`))
  (`self.Game Start`))

(event `Game Start`
  (bind _returnvalue (`KismetSystemLibrary.K2_SetTimerDelegate` (delegate `LoseOutOfTime`) (`self.StartTimerDuration`)))
  (set `self.TimeRemainingTimer` _returnvalue))

(event `LoseOutOfTime`
  (`self.Game Finish` false))

(event `WinCrossedFinishLine`
  (`KismetSystemLibrary.K2_ClearAndInvalidateTimerHandle` (`self.TimeRemainingTimer`))
  (`self.Game Finish` true))

(event `Game Finish`
  (params (bWin :type Boolean))
  (`KismetSystemLibrary.PrintString` (`KismetMathLibrary.SelectString` "Win" "Lose" bWin)))

(event `CrossedCheckpoint`
  (params (GivenTime :type Integer))
  (`self.AddTimeToTimer` GivenTime))

(fn `AddTimeToTimer`
  (params (TimeToAdd :type Integer))
  (set `self.StartTimerDuration` (+ (`local.TimeToAdd`) (`self.StartTimerDuration`))))

(fn `UserConstructionScript`)